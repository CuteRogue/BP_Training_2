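; Player pawn that rolls its static mesh by applying torque from move input and restarts the level when damaged.
; Damage is handled once and branches on the causer: projectiles play a red overlay timeline before a white fade, the finish trigger gives a slower black fade, anything else fades quickly to white.
; A shared Restart Level routine fades the camera, waits, then reopens the current level; BeginPlay fades back in.
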(event `self.ReceiveBeginPlay`
  (`PlayerCameraManager.StartCameraFade` :`self` (`GameplayStatics.GetPlayerCameraManager` 0) :`FromAlpha` 1.0 :`Duration` 2.0 :`bShouldFadeAudio` true :`bHoldWhenFinished` true))

(event `InputAxis|MoveForward`
  (params (AxisValue :type "Float (single-precision)"))
  (`PrimitiveComponent.AddTorqueInRadians` (`self.StaticMesh`) (`KismetMathLibrary.MakeVector` 0.0 (* AxisValue (`self.Acceleration`))) "None" true))

(event `InputAxis|MoveRight`
  (params (AxisValue :type "Float (single-precision)"))
  (`PrimitiveComponent.AddTorqueInRadians` (`self.StaticMesh`) (`KismetMathLibrary.MakeVector` (* (* AxisValue (`self.Acceleration`)) -1.0)) "None" true))

(event `self.ReceiveAnyDamage`
  (params (Damage :type "Float (single-precision)") (DamageType :type "DamageType Object Reference") (InstigatedBy :type "Controller Object Reference") (DamageCauser :type "Actor Object Reference"))
  (`/Engine/EditorBlueprintResources/StandardMacros.DoOnce` false
    (:`Completed`
      (`/Game/Blueprints/Library/CC_MacroLibrary.Validate Class` DamageCauser "/Game/Blueprints/Actors/Projectiles/BP_Projectile.BP_Projectile_C"
        (:`Valid Class`
          (bind (_direction _overlay_value) (`Timeline|Damage Effect` :!via `PlayFromStart`)
            (:`Update`
              (`self.Set Camera Fade` _overlay_value))
            (:`Finished`
              (`self.Restart Level` (struct :`R` 1.0 :`G` 1.0 :`B` 1.0 :`A` 1.0) 0.5 :!label _label))))
        (:`Other`
          (`/Game/Blueprints/Library/CC_MacroLibrary.Validate Class` DamageCauser "/Game/Blueprints/Actors/LevelTriggers/BP_FinishTrigger.BP_FinishTrigger_C"
            (:`Valid Class`
              (`self.Restart Level` (struct) 2.0))
            (:`Other`
              (goto _label))))))))

(fn `Set Camera Fade`
  (params (InFadeAmount :type "Float (single-precision)"))
  (`PlayerCameraManager.SetManualCameraFade` (`GameplayStatics.GetPlayerCameraManager` 0) InFadeAmount (struct :`R` 1.0 :`B` 0.041492 :`A` 1.0) false))

(fn `UserConstructionScript`)