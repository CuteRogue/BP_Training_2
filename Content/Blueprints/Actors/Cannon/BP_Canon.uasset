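; BP_Canon is a cannon actor that fires projectiles automatically in an endless loop from BeginPlay.
; After a FIreDelay wait, it spawns a BP_Projectile at the Arrow component's transform, scaled by ProjectileScale, and plays the AnimateShoot timeline.
; The timeline slides the Cannon component along relative Y for the barrel motion, and its Canon Fired track restarts the delay and fire cycle.
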(event `self.ReceiveBeginPlay`
  (`KismetSystemLibrary.Delay` (`self.FIre Delay`) :!label _label)
  (`self.Spawn Projectile`)
  (bind (_direction _barrel_position) (`Timeline|Animate Shoot` :!via `PlayFromStart`)
    (:`Update`
      (`self.Move Barrel` _barrel_position))
    (:`Canon Fired`
      (goto _label))))

(fn `Move Barrel`
  (params (NewLocation_Y :type "Float (double-precision)"))
  (`SceneComponent.K2_SetRelativeLocation` (`self.Cannon`) (`KismetMathLibrary.MakeVector` 0.0 NewLocation_Y) false false))

(fn `Spawn Projectile`
  (bind (_returnvalue_location _returnvalue_rotation) (`KismetMathLibrary.BreakTransform` (`SceneComponent.K2_GetComponentToWorld` (`self.Arrow`))))
  (`|SpawnActorFromClass` "/Game/Blueprints/Actors/Projectiles/BP_Projectile.BP_Projectile_C" (`KismetMathLibrary.MakeTransform` _returnvalue_location _returnvalue_rotation (`KismetMathLibrary.Conv_DoubleToVector` (`self.Projectile Scale`))) "Undefined" "MultiplyWithRoot" null null))

(fn `UserConstructionScript`)