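; BP_Crystal is a collectible crystal actor that flies into the player and vanishes when the player overlaps it.
; On BeginPlay it caches its starting location, scale and point light intensity.
; A validated player overlap plays CollectionTimeline, whose separate tracks lerp location toward the pawn's current position and fade scale and light intensity to zero.
; The actor destroys itself when the timeline finishes.
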(event `self.ReceiveBeginPlay`
  (`self.Init`))

(event `self.ReceiveActorBeginOverlap`
  (params (OtherActor :type "Actor Object Reference"))
  (bind _pawn (`/Game/Blueprints/Library/CC_MacroLibrary.Validate Player Pawn` OtherActor)
    (:`Player`
      (bind (_direction _collection_progress _collection_scale_progress _collection_light_intensity) (`Timeline|Collection Timeline`)
        (:`Update`
          (`self.Lerp Position` _pawn _collection_progress)
          (`self.Lerp Scale` _collection_scale_progress)
          (`self.Lerp Light Intensity` _collection_light_intensity))
        (:`Finished`
          (`self.K2_DestroyActor`))))))

(fn `Init`
  (set `self.Start Location` (`self.K2_GetActorLocation`))
  (set `self.Start Scale` (`self.GetActorScale3D`))
  (set `self.Start Light Intensity` (`LightComponentBase.Intensity` (`self.PointLight`))))

(fn `Lerp Light Intensity`
  (params (Alpha :type "Float (double-precision)"))
  (`LightComponent.SetIntensity` (`self.PointLight`) (`KismetMathLibrary.Lerp` (`self.Start Light Intensity`) 0.0 Alpha)))

(fn `Lerp Position`
  (params (PlayerPawn :type "Pawn Object Reference") (`Collection Progress` :type "Float (double-precision)"))
  (`self.K2_SetActorLocation` (`KismetMathLibrary.VLerp` (`self.Start Location`) (`self.K2_GetActorLocation` PlayerPawn) `Collection Progress`)))

(fn `Lerp Scale`
  (params (Alpha :type "Float (single-precision)"))
  (`self.SetActorScale3D` (`KismetMathLibrary.VLerp` (`self.Start Scale`) (0.0 0.0 0.0) Alpha)))

(fn `UserConstructionScript`)