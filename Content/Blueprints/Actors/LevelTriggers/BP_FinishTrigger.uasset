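; Finish-line trigger actor that damages the player on overlap while any crystals remain in the level.
; On begin overlap it filters for the player pawn, then checks AnyCrystalRemaining, which searches the level for BP_Crystal actors.
; If crystals remain, it applies damage to the pawn with itself as causer.
; The no-crystals branch also calls ApplyDamage, but with no damaged actor set.
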(event `self.ReceiveActorBeginOverlap`
  (params (OtherActor :type "Actor Object Reference"))
  (bind _pawn (`/Game/Blueprints/Library/CC_MacroLibrary.Validate Player Pawn` OtherActor)
    (:`Player`
      (if (`self.AnyCrystalRemaining`)
        (`GameplayStatics.ApplyDamage` _pawn 1.0 null self)
        (else
          (`GameplayStatics.ApplyDamage` null 1.0))))))

(fn `AnyCrystalRemaining`
  (returns (ReturnValue :type Boolean))
  (bind _outactors (`GameplayStatics.GetAllActorsOfClass` "/Game/Blueprints/Actors/Collectibles/BP_Crystal.BP_Crystal_C"))
  (return (> (`KismetArrayLibrary.Array_Length` _outactors) 0)))

(fn `UserConstructionScript`)